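; BP_Enemy is a sword-wielding enemy character that exposes movement and attack events, none of which are called within this graph.
; Run and Walk switch the CharacterMovement max walk speed between a fast and a slow pace.
; Attack plays a slash animation directly on the mesh, then restores Animation Blueprint mode after a fixed delay.
; The construction script attaches the Sword component to the mesh's SwordSocket.
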(event `Run`
  (set `CharacterMovementComponent.MaxWalkSpeed` 450.0 (`self.CharacterMovement`)))

(event `Walk`
  (set `CharacterMovementComponent.MaxWalkSpeed` 150.0 (`self.CharacterMovement`)))

(event `Attack`
  (`SkeletalMeshComponent.PlayAnimation` (`self.Mesh`) "/Game/Project/Animations/Sword_and_Shield_Pack/sword_and_shield_slash.sword_and_shield_slash" false)
  (`KismetSystemLibrary.Delay` 1.2)
  (`SkeletalMeshComponent.SetAnimationMode` (`self.Mesh`) "AnimationBlueprint"))

(fn `UserConstructionScript`
  (`SceneComponent.K2_AttachToComponent` (`self.Sword`) (`self.Mesh`) "SwordSocket" "KeepRelative" "KeepRelative" "KeepRelative" true))