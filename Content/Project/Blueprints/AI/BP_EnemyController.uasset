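; BP_EnemyController is the AI controller for BP_Enemy, running BT_Enemy on possession and forwarding stun, attack, walk, run and death calls to the pawn.
; Perception updates for the player set the Detected blackboard key, and losing the player stores their current location as an alerted position.
; Rock alerts within AlertRadius also set the alerted position.
; Stun flags the blackboard, and death stops the behavior tree logic.
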(event `Stun`
  (`BlackboardComponent.SetValueAsBool` (`AIBlueprintHelperLibrary.GetBlackboard` null) (`self.StunnedKey`) true)
  (`/Game/Project/Blueprints/AI/BP_Enemy.Stun` (`self.Enemy`)))

(event `Attack`
  (`/Game/Project/Blueprints/AI/BP_Enemy.Attack` (`self.Enemy`)))

(event `Walk`
  (`/Game/Project/Blueprints/AI/BP_Enemy.Walk` (`self.Enemy`)))

(event `Run`
  (`/Game/Project/Blueprints/AI/BP_Enemy.Run` (`self.Enemy`)))

(event `self.ReceivePossess`
  (params (PossessedPawn :type "Pawn Object Reference"))
  (bind _asbp_enemy (cast `/Game/Project/Blueprints/AI/BP_Enemy` PossessedPawn))
  (set `self.Enemy` _asbp_enemy)
  (`self.RunBehaviorTree` "/Game/Project/Blueprints/AI/BT_Enemy.BT_Enemy"))

(event `self.AIPerception.OnTargetPerceptionUpdated`
  (params (Actor :type "Actor Object Reference") (Stimulus :type "AIStimulus Structure"))
  (bind (_age _expirationage _strength _stimuluslocation _receiverlocation _tag _bsuccessfullysensed) (break `AIStimulus` Stimulus))
  (bind _returnvalue (`AIBlueprintHelperLibrary.GetBlackboard` null))
  (if (== (`GameplayStatics.GetPlayerPawn` 0) Actor)
    (`BlackboardComponent.SetValueAsBool` _returnvalue (`self.Detected Key`) _bsuccessfullysensed)
    (if (not _bsuccessfullysensed)
      (`BlackboardComponent.SetValueAsVector` _returnvalue (`self.AlertedPosKey`) (`self.K2_GetActorLocation` (`GameplayStatics.GetPlayerPawn` 0)))
      (`BlackboardComponent.SetValueAsBool` _returnvalue (`self.AlertedKey`) true))))

(event `OnRockAlert`
  (params (Position :type "Vector Structure"))
  (bind _returnvalue (`AIBlueprintHelperLibrary.GetBlackboard` null))
  (if (<= (`KismetMathLibrary.VSize` (- Position (`self.K2_GetActorLocation` (`self.Enemy`)))) (`self.AlertRadius`))
    (`BlackboardComponent.SetValueAsVector` _returnvalue (`self.AlertedPosKey`) Position)
    (`BlackboardComponent.SetValueAsBool` _returnvalue (`self.AlertedKey`) true)))

(event `Death`
  (`BrainComponent.StopLogic` (`self.BrainComponent`) "")
  (`/Game/Project/Blueprints/AI/BP_Enemy.Death` (`self.Enemy`)))

(fn `UserConstructionScript`)