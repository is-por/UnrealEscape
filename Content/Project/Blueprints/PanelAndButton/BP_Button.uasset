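; Push button actor that toggles between pressed and released when something overlaps its box, likely a hand-operated control.
; When in a panel, it responds only to "Hand"-tagged components while the panel is active, and pulses the panel; standalone, any overlap triggers it.
; Each toggle swaps the material, plays a sound and slides the mesh between its initial position and one lowered by the arrow's length.
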(event `self.ReceiveBeginPlay`
  (bind _button (`self.Button`))
  (bind _returnvalue_location (`KismetMathLibrary.BreakTransform` (`SceneComponent.GetRelativeTransform` _button)))
  (`|ExecutionSequence`
    (:`then_0`
      (set `self.length` (`ArrowComponent.ArrowLength` (`self.Arrow`))))
    (:`then_1`
      (set `self.InitPos` _returnvalue_location)
      (set `self.EndPos` (- _returnvalue_location (`KismetMathLibrary.MakeVector` 0.0 0.0 (`self.length`)))))
    (:`then_2`
      (set `self.InitMaterial` (`|GetArrayItem` (`MeshComponent.GetMaterials` _button))))))

(event `self.Box.OnComponentBeginOverlap`
  (params (OverlappedComponent :type "PrimitiveComponent Object Reference") (OtherActor :type "Actor Object Reference") (OtherComp :type "PrimitiveComponent Object Reference") (OtherBodyIndex :type Integer) (bFromSweep :type Boolean) (SweepResult :type "HitResult Structure (by ref)"))
  (bind _button (`self.Button`))
  (if (`self.IsInPanel`)
    (if (and (`ActorComponent.ComponentHasTag` OtherComp "Hand") (`/Game/Project/Blueprints/PanelAndButton/BP_Panel.isActive` (`self.BP_Panel`)))
      (set `self.DestinyPos` (`self.InitPos`) :!label _label)
      (if (`self.isPressed`)
        (`PrimitiveComponent.SetMaterial` _button 0 (`self.InitMaterial`))
        (else
          (`PrimitiveComponent.SetMaterial` _button 0 (`self.PressMaterial`))
          (set `self.DestinyPos` (`self.EndPos`))))
      (`GameplayStatics.PlaySound2D` (`self.SoundPush`) 2.0 1.2 0.0 null null)
      (`KismetSystemLibrary.MoveComponentTo` (`self.Button`) (`self.DestinyPos`) (struct) false false 0.5)
      (set `self.isPressed` (not (`self.isPressed`)))
      (if (`self.IsInPanel`)
        (`/Game/Project/Blueprints/PanelAndButton/BP_Panel.PulseButton` (`self.BP_Panel`))))
    (else
      (goto _label))))

(fn `UserConstructionScript`)