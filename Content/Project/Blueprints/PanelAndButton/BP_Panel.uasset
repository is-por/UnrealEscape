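; BP_Panel is a puzzle panel that checks a set of buttons against a required pressed-state pattern and opens doors when it matches.
; PulseButton compares each button's IsPressed to the CorrectButtons map by button ID, stopping at the first mismatch.
; On a full match it sets IsCompleted, swaps the cube to a completed material and sends ActivateMessage to each linked automatic door.
; A separate Activate event only sets IsActive.
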(event `PulseButton`
  (for _array_element (`self.ArrayButtons`)
    (if (== (`/Game/Project/Blueprints/PanelAndButton/BP_Button.isPressed` _array_element) (`BlueprintMapLibrary.Map_Find` (`self.CorrectButtons`) (`/Game/Project/Blueprints/PanelAndButton/BP_Button.IDButton` _array_element)))
      (set `self.IsBreak` false)
      (else
        (set `self.IsBreak` true)
        (break))))
  (if (not (`self.IsBreak`))
    (set `self.IsCompleted` true)
    (`PrimitiveComponent.SetMaterial` (`self.Cube`) 0 (`self.MaterialCompleted`))
    (for _array_element_2 (`self.Bp_Automatic_Door`)
      (message `/Game/Project/Blueprints/Palanca/BI_Activable.Activate` _array_element_2))))

(event `/Game/Project/Blueprints/Palanca/BI_Activable.Activate`
  (set `self.isActive` true))

(fn `UserConstructionScript`)