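; BP_Automatic_Door is a door that slides to an open position when it receives a PanelComplete event.
; On BeginPlay it reads the length of an Arrow component and sets the end position that far below the door's starting relative location.
; PanelComplete moves the Dooor component to that position over a short fixed time, with no closing logic.
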(event `self.ReceiveBeginPlay`
  (bind _returnvalue_location (`KismetMathLibrary.BreakTransform` (`SceneComponent.GetRelativeTransform` (`self.Dooor`))))
  (`|ExecutionSequence`
    (:`then_0`
      (set `self.length` (`ArrowComponent.ArrowLength` (`self.Arrow`))))
    (:`then_1`
      (set `self.EndPos` (- _returnvalue_location (`KismetMathLibrary.MakeVector` 0.0 0.0 (`self.length`)))))))

(event `PanelComplete`
  (`KismetSystemLibrary.MoveComponentTo` (`self.Dooor`) (`self.EndPos`) (struct) false false 0.5))

(fn `UserConstructionScript`)