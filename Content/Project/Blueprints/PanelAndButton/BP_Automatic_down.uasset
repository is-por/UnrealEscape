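; Automatic door that toggles between a lowered position and its relative origin each time Activate is called.
; On BeginPlay, the Arrow component's length sets the drop distance, and the lowered target is computed from the door's starting relative location.
; Activate uses MoveComponentTo for a timed slide and tracks the state with IsEnd; the return move targets relative zero, as no start position is stored.
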(event `self.ReceiveBeginPlay`
  (bind _returnvalue_location (`KismetMathLibrary.BreakTransform` (`SceneComponent.GetRelativeTransform` (`self.Dooor`))))
  (`|ExecutionSequence`
    (:`then_0`
      (set `self.length` (`ArrowComponent.ArrowLength` (`self.Arrow`))))
    (:`then_1`
      (set `self.EndPos` (- _returnvalue_location (`KismetMathLibrary.MakeVector` 0.0 0.0 (`self.length`)))))))

(event `Activate`
  (if (not (`self.IsEnd`))
    (`KismetSystemLibrary.MoveComponentTo` (`self.Dooor`) (`self.EndPos`) (struct) false false 2.0)
    (set `self.IsEnd` (not (`self.IsEnd`)))
    (else
      (`KismetSystemLibrary.MoveComponentTo` (`self.Dooor`) (0.0 0.0 0.0) (struct) false false 2.0)
      (set `self.IsEnd` false))))

(fn `UserConstructionScript`)