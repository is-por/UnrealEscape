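; Throwable rock interactable that alerts enemies to its position when it hits the floor.
; When its GrabComponent drops it, the mesh gets a velocity-change impulse scaled from its current velocity by Impulso.
; A hit on a component tagged "floor" calls OnRockAlert with the rock's location on every BP_EnemyController.
; The ControlCollision flag blocks repeated hit handling until a short delay resets it.
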(event `Event Dropped`
  (bind _staticmesh (`self.StaticMesh`))
  ;[1 1 1] Impulso tras soltar la piedra
  (`PrimitiveComponent.AddImpulse` _staticmesh (* (`SceneComponent.GetComponentVelocity` _staticmesh) (`self.Impulso`)) "None" true))

(event `self.ReceiveBeginPlay`
  (set `self.controlCollision` false)
  ;[1 1 1] Impulso tras soltar la piedra
  (add `/Game/External/VRTemplate/Blueprints/GrabComponent.OnDropped` (`self.GrabComponent`) (delegate `Event Dropped`)))

(event `self.ReceiveHit`
  (params (MyComp :type "PrimitiveComponent Object Reference") (Other :type "Actor Object Reference") (OtherComp :type "PrimitiveComponent Object Reference") (bSelfMoved :type Boolean) (HitLocation :type "Vector Structure") (HitNormal :type "Vector Structure") (NormalImpulse :type "Vector Structure") (Hit :type "HitResult Structure (by ref)"))
  ;[1 1 1] Comprobamos si colisionamos con el suelo
  (if (not (`self.controlCollision`))
    (set `self.controlCollision` true)
    (if (`ActorComponent.ComponentHasTag` OtherComp "floor")
      (bind _outactors (`GameplayStatics.GetAllActorsOfClass` "/Game/Project/Blueprints/AI/BP_EnemyController.BP_EnemyController_C"))
      (for _array_element _outactors
        (`/Game/Project/Blueprints/AI/BP_EnemyController.OnRockAlert` _array_element (`self.K2_GetActorLocation`))
        (`KismetSystemLibrary.Delay` 1.5 :!label _label)
        (set `self.controlCollision` false))
      (else
        (goto _label)))))

(fn `UserConstructionScript`)