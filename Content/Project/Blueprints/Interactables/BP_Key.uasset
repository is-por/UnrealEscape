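; BP_Key is a grabbable key interactable that signals a door when dropped inside it.
; BeginPlay clears InDoor and caches the initial relative scale, which is restored each time GrabComponent reports a grab.
; On drop with InDoor set, it calls KeyInDoorEvent on AutomaticDoor if valid, otherwise on GrabDoor.
; Nothing in this Blueprint sets InDoor true or assigns the door references.
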(event `self.GrabComponent.OnGrabbed`
  (params (IsHandL :type Boolean) (`Hand Reference` :type "SceneComponent Object Reference"))
  (`self.SetActorRelativeScale3D` self (`self.InitialScale`)))

(event `self.GrabComponent.OnDropped`
  (bind _automaticdoor (`self.automaticDoor`))
  (bind _grabdoor (`self.grabDoor`))
  (if (`self.inDoor`)
    (`/Engine/EditorBlueprintResources/StandardMacros.IsValid` _automaticdoor
      (:`Is Valid`
        (`/Game/Project/Blueprints/Door/BP_door.KeyInDoor_Event` _automaticdoor))
      (:`Is Not Valid`
        (`/Engine/EditorBlueprintResources/StandardMacros.IsValid` _grabdoor
          (:`Is Valid`
            (`KismetSystemLibrary.PrintString` "Hello")
            (`/Game/Project/Blueprints/Door/BP_door_Grab.KeyInDoor_Event` _grabdoor)))))))

(event `self.ReceiveBeginPlay`
  (set `self.inDoor` false)
  (set `self.InitialScale` (`self.GetActorRelativeScale3D` self)))

(fn `UserConstructionScript`)