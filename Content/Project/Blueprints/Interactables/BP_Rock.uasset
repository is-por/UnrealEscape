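; BP_Rock is a grabbable, throwable rock that alerts enemies when it lands.
; Grabbing arms collision detection, and dropping adds a velocity-change impulse scaled from the mesh's current velocity to boost the throw.
; While armed, hits play an alert sound, and floor-tagged hits send the rock's location to every BP_EnemyController through OnRockAlert, disarming it once a valid controller is notified.
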(event `Event Dropped`
  (bind _staticmesh (`self.StaticMesh`))
  ;[1 1 1] Impulso tras soltar la piedra
  (`PrimitiveComponent.AddImpulse` _staticmesh (* (`SceneComponent.GetComponentVelocity` _staticmesh) (`self.Impulso`)) "None" true))

(event `self.ReceiveBeginPlay`
  (set `self.controlCollision` false)
  ;[1 1 1] Impulso tras soltar la piedra
  (add `/Game/External/VRTemplate/Blueprints/GrabComponent.OnDropped` (`self.GrabComponent`) (delegate `Event Dropped`)))

(event `self.ReceiveHit`
  (params (MyComp :type "PrimitiveComponent Object Reference") (Other :type "Actor Object Reference") (OtherComp :type "PrimitiveComponent Object Reference") (bSelfMoved :type Boolean) (HitLocation :type "Vector Structure") (HitNormal :type "Vector Structure") (NormalImpulse :type "Vector Structure") (Hit :type "HitResult Structure (by ref)"))
  ;[1 1 1] Comprobamos si colisionamos con el suelo
  (if (`self.controlCollision`)
    (`GameplayStatics.PlaySound2D` (`self.SoundRockAlert`) 0.5 1.2 0.85 null null)
    (if (`ActorComponent.ComponentHasTag` OtherComp "floor")
      (bind _outactors (`GameplayStatics.GetAllActorsOfClass` "/Game/Project/Blueprints/AI/BP_EnemyController.BP_EnemyController_C"))
      (for _array_element _outactors
        (`/Engine/EditorBlueprintResources/StandardMacros.IsValid` _array_element
          (:`Is Valid`
            (`/Game/Project/Blueprints/AI/BP_EnemyController.OnRockAlert` _array_element (`self.K2_GetActorLocation`))
            (set `self.controlCollision` false)))))))

(event `self.GrabComponent.OnGrabbed`
  (params (IsHandL :type Boolean) (`Hand Reference` :type "SceneComponent Object Reference"))
  (set `self.controlCollision` true))

(fn `UserConstructionScript`)