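; Turret projectile that damages living entities, bounces off shields and destroys itself when its lifetime runs out.
; On overlap with a BP_Shield, it mirrors its forward vector about the shield's right vector and applies that through ProjectileMovement in local space, preserving speed.
; Other actors implementing BI_LivingEntity receive OnDamage and the projectile is destroyed; all other overlaps are ignored.
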(event `self.ReceiveBeginPlay`
  (`KismetSystemLibrary.Delay` (`self.lifetime`))
  (`self.K2_DestroyActor`))

(event `self.ReceiveActorBeginOverlap`
  (params (OtherActor :type "Actor Object Reference"))
  (bind _projectilemovement (`self.ProjectileMovement`))
  (bind _asbp_shield (cast `/Game/Project/Blueprints/Interactables/BP_Shield` OtherActor)
    (:`then`
      (`ProjectileMovementComponent.SetVelocityInLocalSpace` _projectilemovement (`KismetMathLibrary.InverseTransformDirection` (`self.GetTransform`) (* (`KismetMathLibrary.VSize` (`MovementComponent.Velocity` _projectilemovement)) (`KismetMathLibrary.GetReflectionVector` (`self.GetActorForwardVector`) (`self.GetActorRightVector` _asbp_shield))))))
    (:`CastFailed`
      (bind _asbi_living_entity (cast `/Game/Project/Blueprints/BI_LivingEntity` OtherActor))
      (`/Game/Project/Blueprints/BI_LivingEntity.OnDamage` _asbi_living_entity (`self.damage`))
      (`self.K2_DestroyActor`))))

(fn `UserConstructionScript`)