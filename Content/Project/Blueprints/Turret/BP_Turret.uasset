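; BP_Turret is a turret actor that can take damage and die, delegating turret behavior to an ACTurretComponent.
; The construction script hands the component the Gun as its head and a Scene component as the projectile exit.
; Health starts at MaxHealth and drops only when destructible, with damage and break sounds.
; At zero health, death plays a fire sound, marks the component not alive and activates a particle system.
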(event `self.ReceiveBeginPlay`
  (set `self.health` (`self.max health`)))

(event `self.OnDamage`
  (params (damage :type "Float (double-precision)"))
  (if (`self.IsDestructible`)
    (`GameplayStatics.PlaySound2D` (`self.SoundMonsterDamage`) 0.5 1.2 0.0 null null)
    (bind _output_get (set `self.health` (`KismetMathLibrary.FClamp` (- (`self.health`) damage) 0.0 (`self.max health`))))
    (if (<= _output_get 0.0)
      (`GameplayStatics.PlaySound2D` (`self.SoundBreak`) 0.5 1.2 0.0 null null)
      (`self.OnDeath`))))

(event `self.OnDeath`
  (`GameplayStatics.PlaySound2D` (`self.SoundFire`) 0.5 1.2 0.0 null null)
  (set `/Game/Project/Blueprints/Turret/AC_TurretComponent.alive` false (`self.AC_TurretComponent`))
  (`ActorComponent.Activate` (`self.ParticleSystem`) false))

(fn `UserConstructionScript`
  (bind _ac_turretcomponent (`self.AC_TurretComponent`))
  (set `/Game/Project/Blueprints/Turret/AC_TurretComponent.Head` (`self.Gun`) _ac_turretcomponent)
  (set `/Game/Project/Blueprints/Turret/AC_TurretComponent.ProjectileExit` (`self.Scene`) _ac_turretcomponent))