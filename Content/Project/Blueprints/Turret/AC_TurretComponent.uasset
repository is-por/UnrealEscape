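; Turret actor component that makes its owner track and fire at the player pawn.
; Each tick, while alive and the player is between a fixed minimum distance and SightDistance, it interpolates the Head's relative rotation toward a look-at from ProjectileExit.
; An accumulated timer fires at ShootFreq shots per second, spawning BP_Projectile at ProjectileExit and playing a 2D sound.
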(event `self.ReceiveTick`
  (params (DeltaSeconds :type "Float (single-precision)"))
  (bind _returnvalue (`Actor.K2_GetActorLocation` (`GameplayStatics.GetPlayerPawn` 0)))
  (bind _returnvalue_2 (`KismetMathLibrary.Vector_Distance` (`Actor.K2_GetActorLocation` (`self.GetOwner`)) _returnvalue))
  (if (and (`self.alive`) (and (>= _returnvalue_2 200.0) (<= _returnvalue_2 (`self.sightDistance`))))
    (`self.UpdateLookAt` _returnvalue DeltaSeconds)
    (`self.Shoot` DeltaSeconds)))

(fn `Shoot`
  (params (deltaTime :type "Float (double-precision)"))
  (bind _output_get (set `self.lastShoot` (+ deltaTime (`self.lastShoot`))))
  (if (>= _output_get (/ 1.0 (`self.shootFreq`)))
    (set `self.lastShoot` 0.0)
    (`|SpawnActorFromClass` "/Game/Project/Blueprints/Turret/BP_Projectile.BP_Projectile_C" (`SceneComponent.K2_GetComponentToWorld` (`self.ProjectileExit`)) "Undefined" "OverrideRootScale" null null)
    (`GameplayStatics.PlaySound2D` (`self.Sound`) 0.5 1.0 0.0 null null)))

(fn `UpdateLookAt`
  (params (LookAt :type "Vector Structure") (deltaTime :type "Float (double-precision)"))
  (bind _head (`self.Head`))
  (`SceneComponent.K2_SetRelativeRotation` _head (`KismetMathLibrary.RInterpTo` (`SceneComponent.RelativeRotation` _head) (`KismetMathLibrary.FindLookAtRotation` (`SceneComponent.K2_GetComponentLocation` (`self.ProjectileExit`)) LookAt) deltaTime (`self.speed`)) false false))