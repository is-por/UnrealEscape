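; BulletRecollector is an actor that absorbs projectiles and triggers linked objects once enough have been collected.
; Each BP_Projectile overlapping its Sphere1 component is destroyed and increments a counter.
; When the counter reaches BulletsForComplete, it latches complete, swaps the Sphere material, and sends ActivateMessage to ActivateObjects and OnDeathMessage to KillEnemies.
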(event `self.Sphere1.OnComponentBeginOverlap`
  (params (OverlappedComponent :type "PrimitiveComponent Object Reference") (OtherActor :type "Actor Object Reference") (OtherComp :type "PrimitiveComponent Object Reference") (OtherBodyIndex :type Integer) (bFromSweep :type Boolean) (SweepResult :type "HitResult Structure (by ref)"))
  (cast `/Game/Project/Blueprints/Turret/BP_Projectile` OtherActor)
  (`/Engine/EditorBlueprintResources/StandardMacros.IncrementInt` (`self.CounterBullets`)
    (:`  `
      (`self.K2_DestroyActor` OtherActor)
      (if (and (>= (`self.CounterBullets`) (`self.BulletsForComplete`)) (not (`self.isComplete`)))
        (set `self.isComplete` true)
        (`PrimitiveComponent.SetMaterial` (`self.Sphere`) 0 (`self.M_MaterialComplete`))
        (for _array_element (`self.ActivateObjects`)
          (message `/Game/Project/Blueprints/Palanca/BI_Activable.Activate` _array_element))
        (for _array_element_2 (`self.KillEnemies`)
          (message `/Game/Project/Blueprints/BI_LivingEntity.OnDeath` _array_element_2))))))

(fn `UserConstructionScript`)