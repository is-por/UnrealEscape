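; BP_ComponentDoor is a door that accepts one specific BP_Key.
; Its box collider sets InDoor on that key when overlap begins and clears it on any BP_Key when overlap ends.
; KeyInDoor_Event, not called within this graph, prints a door-open message and snaps the key to the KeySocket on the door mesh, without moving the door itself.
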(event `self.ReceiveBeginPlay`
  (bind _boxcollider (`self.BoxCollider`))
  (`|ExecutionSequence`
    (:`then_0`
      (add `PrimitiveComponent.OnComponentBeginOverlap` _boxcollider (delegate `OnComponentBeginOverlap_Event_0`)))
    (:`then_1`
      (add `PrimitiveComponent.OnComponentEndOverlap` _boxcollider (delegate `OnComponentEndOverlap_Event_0`)))))

(event `OnComponentBeginOverlap_Event_0`
  (params (OverlappedComponent :type "PrimitiveComponent Object Reference") (OtherActor :type "Actor Object Reference") (OtherComp :type "PrimitiveComponent Object Reference") (OtherBodyIndex :type Integer) (bFromSweep :type Boolean) (SweepResult :type "HitResult Structure (by ref)"))
  (bind _asbp_key (cast `/Game/Project/Blueprints/Interactables/BP_Key` OtherActor))
  (if (== _asbp_key (`self.Key`))
    (set `/Game/Project/Blueprints/Interactables/BP_Key.inDoor` true _asbp_key)))

(event `OnComponentEndOverlap_Event_0`
  (params (OverlappedComponent :type "PrimitiveComponent Object Reference") (OtherActor :type "Actor Object Reference") (OtherComp :type "PrimitiveComponent Object Reference") (OtherBodyIndex :type Integer))
  (bind _asbp_key (cast `/Game/Project/Blueprints/Interactables/BP_Key` OtherActor))
  (set `/Game/Project/Blueprints/Interactables/BP_Key.inDoor` false _asbp_key))

(event `KeyInDoor_Event`
  (`KismetSystemLibrary.PrintString` "Puera abierta")
  (`Actor.K2_AttachToComponent` (`self.key`) (`self.Static Mesh Door`) "KeySocket" "SnapToTarget" "SnapToTarget" "SnapToTarget" true))