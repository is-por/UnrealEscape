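; Door Blueprint that opens with a specific assigned BP_Key.
; BeginPlay sets the mesh, moves the trigger Box to its KeySocket and stores the initial rotation.
; Box overlaps set the matching key's InDoor flag; ending overlap clears it for any BP_Key.
; KeyInDoor_Event, not called within this graph, snaps the key into the socket and plays a timeline adding a scaled DeltaApertura to the starting rotation.
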(event `self.ReceiveBeginPlay`
  (bind _staticmeshdoor (`self.staticMeshDoor`))
  (`|ExecutionSequence`
    (:`then_0`
      (`StaticMeshComponent.SetStaticMesh` (`self.doorStaticMesh`) _staticmeshdoor)
      (`SceneComponent.K2_SetRelativeLocation` (`self.Box`) (`StaticMeshSocket.RelativeLocation` (`StaticMesh.FindSocket` _staticmeshdoor "KeySocket")) false false))
    (:`then_1`
      (set `self.rotacionInicial` (`SceneComponent.RelativeRotation` (`self.doorStaticMesh`))))))

(event `self.Box.OnComponentBeginOverlap`
  (params (OverlappedComponent :type "PrimitiveComponent Object Reference") (OtherActor :type "Actor Object Reference") (OtherComp :type "PrimitiveComponent Object Reference") (OtherBodyIndex :type Integer) (bFromSweep :type Boolean) (SweepResult :type "HitResult Structure (by ref)"))
  (bind _asbp_key (cast `/Game/Project/Blueprints/Interactables/BP_Key` OtherActor))
  (if (== _asbp_key (`self.key`))
    (set `/Game/Project/Blueprints/Interactables/BP_Key.inDoor` true _asbp_key)))

(event `self.Box.OnComponentEndOverlap`
  (params (OverlappedComponent :type "PrimitiveComponent Object Reference") (OtherActor :type "Actor Object Reference") (OtherComp :type "PrimitiveComponent Object Reference") (OtherBodyIndex :type Integer))
  (bind _asbp_key (cast `/Game/Project/Blueprints/Interactables/BP_Key` OtherActor))
  (set `/Game/Project/Blueprints/Interactables/BP_Key.inDoor` false _asbp_key))

(event `KeyInDoor_Event`
  (bind (_deltaapertura_roll _deltaapertura_pitch _deltaapertura_yaw) (`KismetMathLibrary.BreakRotator` (`self.deltaApertura`)))
  (bind (_rotacioninicial_roll _rotacioninicial_pitch _rotacioninicial_yaw) (`KismetMathLibrary.BreakRotator` (`self.rotacionInicial`)))
  (`KismetSystemLibrary.PrintString` "Puera abierta")
  (`self.K2_AttachToComponent` (`self.key`) (`self.doorStaticMesh`) "KeySocket" "SnapToTarget" "SnapToTarget" "SnapToTarget" true)
  (bind (_direction _proporcionapertura) (`Timeline|RotationLerp`)
    (:`Update`
      (bind (_returnvalue_x _returnvalue_y _returnvalue_z) (`KismetMathLibrary.BreakVector` (+ (`KismetMathLibrary.MakeVector` _rotacioninicial_roll _rotacioninicial_pitch _rotacioninicial_yaw) (* _proporcionapertura (`KismetMathLibrary.MakeVector` _deltaapertura_roll _deltaapertura_pitch _deltaapertura_yaw)))))
      (`SceneComponent.K2_SetRelativeRotation` (`self.doorStaticMesh`) (`KismetMathLibrary.MakeRotator` _returnvalue_x _returnvalue_y _returnvalue_z) false false))))

(fn `UserConstructionScript`)