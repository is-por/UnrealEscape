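; VR grabbable hinged door that stays locked until its assigned key is inserted.
; The key box flags overlapping keys as in the door, and KeyInDoor_Event snaps the key to a mesh socket and unlocks it.
; While an open door is grabbed, a gated Tick derives a signed hand-to-pivot angle and updates pivot rotation only within angle limits.
; BeginPlay caches the starting direction and positions both boxes from mesh sockets.
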(event `self.ReceiveBeginPlay`
  (`|ExecutionSequence`
    (:`then_0`
      (set `self.InitDoorDirection` (`SceneComponent.GetRightVector` (`self.DoorPivot`))))
    (:`then_1`
      (`SceneComponent.K2_SetRelativeLocation` (`self.Box`) (`StaticMeshSocket.RelativeLocation` (`StaticMesh.FindSocket` (`StaticMeshComponent.StaticMesh` (`self.DoorStaticMesh`)) "Box")) false false))
    (:`then_2`
      (`SceneComponent.K2_SetRelativeLocation` (`self.GrabBoxSocket`) (`StaticMeshSocket.RelativeLocation` (`StaticMesh.FindSocket` (`StaticMeshComponent.StaticMesh` (`self.DoorStaticMesh`)) "GrabBoxSocket")) false false))))

(event `self.GrabComponent.OnGrabbed`
  (params (IsHandL :type Boolean) (`Hand Reference` :type "SceneComponent Object Reference"))
  (set `self.HandReference` `Hand Reference`)
  (if (`self.IsOpen`)
    (`self.StartTracking`)))

(event `self.GrabComponent.OnDropped`
  (`self.StopTracking`)
  (set `self.HandReference` null))

(event `self.ReceiveTick`
  (params (DeltaSeconds :type "Float (single-precision)"))
  (`/Engine/EditorBlueprintResources/StandardMacros.Gate` true :!label _label
    (:`Exit`
      (set `self.CurrentAngle` (`self.GetDoorAngle`))
      (if (and (<= (`self.CurrentAngle`) (`self.MaxAngle`)) (>= (`self.CurrentAngle`) (`self.MinAngle`)))
        (`SceneComponent.K2_SetWorldRotation` (`self.DoorPivot`) (`KismetMathLibrary.RInterpTo_Constant` (`SceneComponent.K2_GetComponentRotation` (`self.DoorPivot`)) (`self.GetDoorRotation` (0.0 0.0 0.0)) (`GameplayStatics.GetWorldDeltaSeconds`) 100.0) false false)))))

(event `StartTracking`
  (goto _label :!via `Open`))

(event `StopTracking`
  (goto _label :!via `Close`))

(event `self.Box.OnComponentBeginOverlap`
  (params (OverlappedComponent :type "PrimitiveComponent Object Reference") (OtherActor :type "Actor Object Reference") (OtherComp :type "PrimitiveComponent Object Reference") (OtherBodyIndex :type Integer) (bFromSweep :type Boolean) (SweepResult :type "HitResult Structure (by ref)"))
  (`KismetSystemLibrary.PrintString` "Hello")
  (bind _asbp_key (cast `/Game/Project/Blueprints/Interactables/BP_Key` OtherActor))
  (if (== _asbp_key (`self.Key`))
    (set `/Game/Project/Blueprints/Interactables/BP_Key.inDoor` true _asbp_key)))

(event `self.Box.OnComponentEndOverlap`
  (params (OverlappedComponent :type "PrimitiveComponent Object Reference") (OtherActor :type "Actor Object Reference") (OtherComp :type "PrimitiveComponent Object Reference") (OtherBodyIndex :type Integer))
  (bind _asbp_key (cast `/Game/Project/Blueprints/Interactables/BP_Key` OtherActor))
  (set `/Game/Project/Blueprints/Interactables/BP_Key.inDoor` false _asbp_key))

(event `KeyInDoor_Event`
  (`KismetSystemLibrary.PrintString` "Puera abierta")
  (`self.K2_AttachToComponent` (`self.key`) (`self.doorStaticMesh`) "KeySocket" "SnapToTarget" "SnapToTarget" "SnapToTarget" true)
  (set `self.IsOpen` true))

(fn `GetDoorAngle`
  (returns (AngleDoor :type "Float (double-precision)"))
  (bind (_returnvalue_x _returnvalue_y _returnvalue_z) (`KismetMathLibrary.BreakVector` (`KismetMathLibrary.Cross_VectorVector` (`self.GetHandDoorDir`) (`self.InitDoorDirection`))))
  (return (* (`KismetMathLibrary.DegAcos` (`KismetMathLibrary.Dot_VectorVector` (`self.GetHandDoorDir`) (`self.InitDoorDirection`))) (`KismetMathLibrary.SelectFloat` -1.0 1.0 (< _returnvalue_z 0.0)))))

(fn `GetDoorRotation`
  (params (OptionalDirection :type "Vector Structure") (`Use Direction` :type Boolean))
  (returns (Rotation :type "Rotator Structure"))
  (return (`KismetMathLibrary.MakeRotFromYZ` (`KismetMathLibrary.SelectVector` OptionalDirection (`self.GetHandDoorDir`) `Use Direction`) (`SceneComponent.GetUpVector` (`self.DoorPivot`)))))

(fn `GetHandDoorDir`
  (returns (HandDoorDir :type "Vector Structure"))
  (bind (_returnvalue_x _returnvalue_y) (`KismetMathLibrary.BreakVector` (- (`SceneComponent.K2_GetComponentLocation` (`self.HandReference`)) (`SceneComponent.K2_GetComponentLocation` (`self.DoorPivot`)))))
  (return (`KismetMathLibrary.Normal` (`KismetMathLibrary.MakeVector` _returnvalue_x _returnvalue_y))))

(fn `UserConstructionScript`)