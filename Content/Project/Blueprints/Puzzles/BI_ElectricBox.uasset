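; Electric box puzzle where three grabbable connectors (R, G, B) must be plugged into their matching sockets.
; A connector end overlapping any box component snaps and attaches to it, but counts as connected only in its own socket.
; Dropping a socketed connector turns off its physics, and leaving a box clears its state.
; When all three are correctly connected, the puzzle solves once and sends ActivateMessage to each object in ObjectsToActivate.
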(event `self.GrabComponentG.OnDropped`
  (if (`self.inSocketG`)
    (`PrimitiveComponent.SetSimulatePhysics` (`self.SphereEndG`) false)))

(event `self.GrabComponentR.OnDropped`
  (if (`self.inSocketR`)
    (`PrimitiveComponent.SetSimulatePhysics` (`self.SphereEndR`) false)))

(event `self.GrabComponentB.OnDropped`
  (if (`self.inSocketB`)
    (`PrimitiveComponent.SetSimulatePhysics` (`self.SphereEndB`) false)))

(event `self.SphereEndB.OnComponentBeginOverlap`
  (params (OverlappedComponent :type "PrimitiveComponent Object Reference") (OtherActor :type "Actor Object Reference") (OtherComp :type "PrimitiveComponent Object Reference") (OtherBodyIndex :type Integer) (bFromSweep :type Boolean) (SweepResult :type "HitResult Structure (by ref)"))
  (bind (_success _setconnected) (`self.AttachConnector` OverlappedComponent OtherComp (`self.BoxB`)))
  (if _success
    (set `self.inSocketB` true)
    (set `self.ConnectedB` _setconnected)
    (`self.CheckAllConections` :!label _label)))

(event `self.SphereEndR.OnComponentBeginOverlap`
  (params (OverlappedComponent :type "PrimitiveComponent Object Reference") (OtherActor :type "Actor Object Reference") (OtherComp :type "PrimitiveComponent Object Reference") (OtherBodyIndex :type Integer) (bFromSweep :type Boolean) (SweepResult :type "HitResult Structure (by ref)"))
  (bind (_success _setconnected) (`self.AttachConnector` OverlappedComponent OtherComp (`self.BoxR`)))
  (if _success
    (set `self.inSocketR` true)
    (set `self.ConnectedR` _setconnected)
    (goto _label)))

(event `self.SphereEndG.OnComponentBeginOverlap`
  (params (OverlappedComponent :type "PrimitiveComponent Object Reference") (OtherActor :type "Actor Object Reference") (OtherComp :type "PrimitiveComponent Object Reference") (OtherBodyIndex :type Integer) (bFromSweep :type Boolean) (SweepResult :type "HitResult Structure (by ref)"))
  (bind (_success _setconnected) (`self.AttachConnector` OverlappedComponent OtherComp (`self.BoxG`)))
  (if _success
    (set `self.inSocketG` true)
    (set `self.ConnectedG` _setconnected)
    (goto _label)))

(event `self.SphereEndR.OnComponentEndOverlap`
  (params (OverlappedComponent :type "PrimitiveComponent Object Reference") (OtherActor :type "Actor Object Reference") (OtherComp :type "PrimitiveComponent Object Reference") (OtherBodyIndex :type Integer))
  (cast `BoxComponent` OtherComp)
  (set `self.inSocketR` false)
  (set `self.ConnectedR` false))

(event `self.SphereEndB.OnComponentEndOverlap`
  (params (OverlappedComponent :type "PrimitiveComponent Object Reference") (OtherActor :type "Actor Object Reference") (OtherComp :type "PrimitiveComponent Object Reference") (OtherBodyIndex :type Integer))
  (cast `BoxComponent` OtherComp)
  (set `self.inSocketB` false)
  (set `self.ConnectedB` false))

(event `self.SphereEndG.OnComponentEndOverlap`
  (params (OverlappedComponent :type "PrimitiveComponent Object Reference") (OtherActor :type "Actor Object Reference") (OtherComp :type "PrimitiveComponent Object Reference") (OtherBodyIndex :type Integer))
  (cast `BoxComponent` OtherComp)
  (set `self.inSocketG` false)
  (set `self.ConnectedG` false))

(event `OnCompletion`
  (for _array_element (`self.ObjectsToActivate`)
    (message `/Game/Project/Blueprints/Palanca/BI_Activable.Activate` _array_element)))

(fn `AttachConnector`
  (params (Conector :type "PrimitiveComponent Object Reference") (End :type "PrimitiveComponent Object Reference") (BoxTrigger :type "BoxComponent Object Reference"))
  (returns (Success :type Boolean) (SetConnected :type Boolean))
  (bind _asbox_collision (cast `BoxComponent` End)
    (:`then`
      (bind _returnvalue (`SceneComponent.K2_AttachToComponent` Conector _asbox_collision "None" "SnapToTarget" "SnapToTarget" "KeepWorld" true))
      (return _returnvalue (== End BoxTrigger)))
    (:`CastFailed`
      (return false false))))

(fn `CheckAllConections`
  (if (and (`self.ConnectedR`) (`self.ConnectedG`) (`self.ConnectedB`) (not (`self.isSolved`)))
    (set `self.isSolved` true)
    (`self.OnCompletion`)))

(fn `UserConstructionScript`)