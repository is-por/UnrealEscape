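; MySaveData is a save-game object that tracks a game timer's last time and best (lowest) time.
; SaveTimeData records the last time or, on reset, zeroes it and sets the best time to a huge sentinel.
; The best-time comparison and write to the timer slot are unconnected, so nothing is saved.
; LoadTimeData loads that slot but returns GreatTime without reading the loaded object.
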(fn `LoadTimeData`
  (params (Interface :type "/Game/Project/Blueprints/Brazalete/WB_DiegeticInterface Object Reference"))
  (returns (GreatTime :type "Float (double-precision)"))
  (`GameplayStatics.LoadGameFromSlot` "SlotTimerData")
  (return (`self.GreatTime`)))

(fn `SaveTimeData`
  (params (TimeGame :type "Float (double-precision)") (GreatTime :type "Float (double-precision)") (IsReset :type Boolean))
  (if IsReset
    (set `self.LastTime` 0.0)
    (set `self.GreatTime` 1.6666666666666668e+18)
    (else
      (set `self.LastTime` TimeGame))))