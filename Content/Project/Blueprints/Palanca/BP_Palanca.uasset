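; Grabbable lever (palanca) that sends an activate message to linked BPAutomaticDown actors when pulled to a target angle.
; While grabbed, a Tick gate derives a signed angle from the hand's YZ direction around the pivot and sets pivot rotation within limits.
; Reaching the target plays a sound and fires once until the angle drops below it.
; GetCurrentRotation's interpolation node is unconnected, and a key-socket event also sets IsActivate.
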(event `self.ReceiveBeginPlay`
  (set `self.InitDoorDirection` (`SceneComponent.GetUpVector` (`self.DoorPivot`))))

(event `self.GrabComponent.OnGrabbed`
  (params (IsHandL :type Boolean) (`Hand Reference` :type "SceneComponent Object Reference"))
  (set `self.HandReference` `Hand Reference`)
  (`self.StartTracking`))

(event `self.GrabComponent.OnDropped`
  (`self.StopTracking`)
  (set `self.HandReference` null))

(event `self.ReceiveTick`
  (params (DeltaSeconds :type "Float (single-precision)"))
  (`/Engine/EditorBlueprintResources/StandardMacros.Gate` true :!label _label
    (:`Exit`
      (set `self.CurrentAngle` (`self.GetDoorAngle`))
      (if (and (<= (`self.CurrentAngle`) (`self.MaxAngle`)) (>= (`self.CurrentAngle`) (`self.MinAngle`)))
        (`SceneComponent.K2_SetWorldRotation` (`self.DoorPivot`) (`KismetMathLibrary.RInterpTo_Constant` (`SceneComponent.K2_GetComponentRotation` (`self.DoorPivot`)) (`self.GetDoorRotation` (0.0 0.0 0.0)) (`GameplayStatics.GetWorldDeltaSeconds`) 100.0) false false)
        (if (>= (`self.CurrentAngle`) (`self.AngleTarget`))
          (if (not (`self.IsActivate`))
            (for _array_element (`self.BP_AutomaticDown`)
              (message `/Game/Project/Blueprints/Palanca/BI_Activable.Activate` _array_element))
            (set `self.IsActivate` true)
            (`GameplayStatics.PlaySound2D` (`self.SoundPush`) 2.0 1.2 0.0 null null))
          (else
            (set `self.IsActivate` false)))))))

(event `StartTracking`
  (goto _label :!via `Open`))

(event `StopTracking`
  (goto _label :!via `Close`))

(event `KeyInDoor_Event`
  (`self.K2_AttachToComponent` (`self.doorStaticMesh`) "KeySocket" "SnapToTarget" "SnapToTarget" "SnapToTarget")
  (set `self.IsActivate` true))

(fn `Get Hand Door Dir`
  (returns (HandDoorDir :type "Vector Structure"))
  (bind (_returnvalue_x _returnvalue_y _returnvalue_z) (`KismetMathLibrary.BreakVector` (- (`SceneComponent.K2_GetComponentLocation` (`self.HandReference`)) (`SceneComponent.K2_GetComponentLocation` (`self.DoorPivot`)))))
  (return (`KismetMathLibrary.Normal` (`KismetMathLibrary.MakeVector` 0.0 _returnvalue_y _returnvalue_z))))

(fn `GetDoorAngle`
  (returns (AngleDoor :type "Float (double-precision)"))
  (bind (_returnvalue_x _returnvalue_y _returnvalue_z) (`KismetMathLibrary.BreakVector` (`KismetMathLibrary.Cross_VectorVector` (`self.Get Hand Door Dir`) (`self.InitDoorDirection`))))
  (return (* (`KismetMathLibrary.DegAcos` (`KismetMathLibrary.Dot_VectorVector` (`self.Get Hand Door Dir`) (`self.InitDoorDirection`))) (`KismetMathLibrary.SelectFloat` -1.0 1.0 (< _returnvalue_z 0.0)))))

(fn `GetDoorRotation`
  (params (OptionalDirection :type "Vector Structure") (`Use Direction` :type Boolean))
  (returns (Rotation :type "Rotator Structure"))
  (return (`KismetMathLibrary.MakeRotFromZX` (`KismetMathLibrary.SelectVector` OptionalDirection (`self.Get Hand Door Dir`) `Use Direction`) (`SceneComponent.GetForwardVector` (`self.DoorPivot`)))))

(fn `UserConstructionScript`)