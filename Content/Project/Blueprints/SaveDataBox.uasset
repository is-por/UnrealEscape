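; SaveDataBox is a trigger box that records the player's run time as a finish point.
; On BeginPlay it loads best and last times from the SlotTimerData save slot and prints them, or defaults the best time to a huge value when no save exists.
; The first BP_Player overlap creates a fresh MySaveData, passes game time, best time and reset flag to its SaveTimeData, then marks the player finished.
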(event `self.ReceiveBeginPlay`
  (bind _returnvalue (`GameplayStatics.DoesSaveGameExist` "SlotTimerData"))
  (if _returnvalue
    (bind _returnvalue_2 (`GameplayStatics.LoadGameFromSlot` "SlotTimerData"))
    (bind _output_get (set `self.MySaveData` _returnvalue_2))
    (bind _asmy_save_data (cast `/Game/Project/Blueprints/MySaveData` _output_get))
    (bind _output_get_2 (set `self.GreatTime` (`/Game/Project/Blueprints/MySaveData.GreatTime` _asmy_save_data)))
    (`KismetSystemLibrary.PrintString` (`KismetStringLibrary.Conv_DoubleToString` _output_get_2))
    (bind _output_get_3 (set `self.CurrentTime` (`/Game/Project/Blueprints/MySaveData.LastTime` _asmy_save_data)))
    (`KismetSystemLibrary.PrintString` (`KismetStringLibrary.Conv_DoubleToString` _output_get_3))
    (else
      (`KismetSystemLibrary.PrintString` "NO EXISTE")
      (set `self.GreatTime` 16666666666.0))))

(event `self.Box.OnComponentBeginOverlap`
  (params (OverlappedComponent :type "PrimitiveComponent Object Reference") (OtherActor :type "Actor Object Reference") (OtherComp :type "PrimitiveComponent Object Reference") (OtherBodyIndex :type Integer) (bFromSweep :type Boolean) (SweepResult :type "HitResult Structure (by ref)"))
  (bind _asbp_player (cast `/Game/Project/Blueprints/BP_Player` OtherActor))
  (if (not (`/Game/Project/Blueprints/BP_Player.IsFinish` _asbp_player))
    (`GameplayStatics.DoesSaveGameExist` "SlotTimerData")
    (bind _returnvalue (`GameplayStatics.CreateSaveGameObject` "/Game/Project/Blueprints/MySaveData.MySaveData_C"))
    (bind _output_get (set `self.MySaveData` _returnvalue))
    (bind _asmy_save_data (cast `/Game/Project/Blueprints/MySaveData` _output_get))
    (`/Game/Project/Blueprints/MySaveData.SaveTimeData` _asmy_save_data (`/Game/Project/Blueprints/BP_Player.TimeGame` _asbp_player) (`self.GreatTime`) (`self.IsReset`))
    (set `/Game/Project/Blueprints/BP_Player.IsFinish` true _asbp_player)))

(fn `UserConstructionScript`)